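; BP_Clock is an animated clock whose second, minute and hour hand meshes rotate in discrete ticks.
; BeginPlay starts three looping delays: one steps the second hand every second, while the minute and hour timers only set flags.
; The second-hand loop consumes those flags to step the other hands, checking the hour flag only when the minute hand moves.
; Hands advance from their initial rotations, without reading the actual time.
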(event `self.ReceiveBeginPlay`
  ;[1 1 1] Controls how long until rotations
  (`|ExecutionSequence`
    (:`then_0`
      (`KismetSystemLibrary.RetriggerableDelay` 60.0 :!label _label)
      (set `self.MinuteHand` true)
      (goto _label))
    (:`then_1`
      (`KismetSystemLibrary.RetriggerableDelay` 3600.0 :!label _label_2)
      (set `self.HourHand` true)
      (goto _label_2))
    (:`then_2`
      (`KismetSystemLibrary.RetriggerableDelay` 1.0 :!label _label_3)
      (`SceneComponent.K2_AddLocalRotation` (`self.Clock_Second_Hand_SM`) (struct :`Pitch` -6.0) false false)
      (`|ExecutionSequence`
        (:`then_0`
          (goto _label_3))
        (:`then_1`
          (if (`self.MinuteHand`)
            (`SceneComponent.K2_AddLocalRotation` (`self.Clock_Minute_Hand_SM`) (struct :`Pitch` -6.0) false false)
            (set `self.MinuteHand` false)
            (if (`self.HourHand`)
              (`SceneComponent.K2_AddLocalRotation` (`self.Clock_Hour_Hand_SM`) (struct :`Pitch` -30.0) false false)
              (set `self.HourHand` false))))))))

(fn `UserConstructionScript`)